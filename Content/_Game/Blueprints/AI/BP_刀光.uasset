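; BP_刀光 (blade light) is a short-lived AI attack actor that damages the player on overlap.
; When its 刀光 component overlaps an actor tagged 玩家 (player), a DoOnce sends the 受击事件 (hit event) message to that actor.
; The message carries instigator, attack type, hit location, damage and block/attack poise-damage values.
; It destroys itself after that hit, or three seconds after spawning.
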(event `self.ReceiveBeginPlay`
  (`KismetSystemLibrary.Delay` 3.0)
  (`self.K2_DestroyActor`))

(event `self.刀光.OnComponentBeginOverlap`
  (params (OverlappedComponent :type "PrimitiveComponent Object Reference") (OtherActor :type "Actor Object Reference") (OtherComp :type "PrimitiveComponent Object Reference") (OtherBodyIndex :type Integer) (bFromSweep :type Boolean) (SweepResult :type "HitResult Structure (by ref)"))
  (if (`self.ActorHasTag` OtherActor "玩家")
    (`/Engine/EditorBlueprintResources/StandardMacros.IsValid` OtherActor
      (:`Is Valid`
        (`/Engine/EditorBlueprintResources/StandardMacros.DoOnce` false
          (:`Completed`
            (message `/Game/_Game/Data/战斗接口.受击事件` OtherActor (`self.伤害造成者`) (`self.攻击者攻击类型`) (`.Location` (`GameplayStatics.BreakHitResult` SweepResult)) (`self.伤害值`) (`self.格挡削韧值`) (`self.攻击削韧值`))
            (`self.K2_DestroyActor`)))))))

(fn `UserConstructionScript`)