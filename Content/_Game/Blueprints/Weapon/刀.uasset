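; Blade (刀) weapon Blueprint that spawns spark effects for blocks and parries.
; Two notify events each randomize the pitch of one of three attach-point components (3, 4, 5), then spawn a randomly scaled spark system at a randomly selected point.
; Parries use a different effect and larger scale range than blocks.
; Random picks re-roll between nodes, so the rotated point can differ from the spawn point.
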(event `/Game/_Game/Data/战斗接口.通知格挡火花`
  (bind _returnvalue (select `int` (`KismetMathLibrary.RandomIntegerInRange` 0 2) :`0` (`self.3`) :`1` (`self.4`) :`2` (`self.5`)))
  (set `self.火花大小` (`KismetMathLibrary.MakeVector` (`KismetMathLibrary.RandomFloatInRange` 0.5 1.5) (`KismetMathLibrary.RandomFloatInRange` 0.5 1.5) (`KismetMathLibrary.RandomFloatInRange` 0.5 1.5)))
  (`SceneComponent.K2_SetRelativeRotation` _returnvalue (`KismetMathLibrary.MakeRotator` 0.0 (`KismetMathLibrary.RandomFloatInRange` -135.0)) false false)
  (`NiagaraFunctionLibrary.SpawnSystemAtLocation` "/Game/Blood_VFX_Pack/Particles/Parts/P_E_Sparks_01.P_E_Sparks_01" (`SceneComponent.K2_GetComponentLocation` _returnvalue) (`SceneComponent.K2_GetComponentRotation` _returnvalue) (`self.火花大小`)))

(event `/Game/_Game/Data/战斗接口.通知弹反火花`
  (bind _returnvalue (select `int` (`KismetMathLibrary.RandomIntegerInRange` 0 2) :`0` (`self.3`) :`1` (`self.4`) :`2` (`self.5`)))
  (set `self.火花大小` (`KismetMathLibrary.MakeVector` (`KismetMathLibrary.RandomFloatInRange` 1.0 2.0) (`KismetMathLibrary.RandomFloatInRange` 1.0 2.0) (`KismetMathLibrary.RandomFloatInRange` 1.0 2.0)))
  (`SceneComponent.K2_SetRelativeRotation` _returnvalue (`KismetMathLibrary.MakeRotator` 0.0 (`KismetMathLibrary.RandomFloatInRange` -135.0)) false false)
  (`NiagaraFunctionLibrary.SpawnSystemAtLocation` "/Game/Blood_VFX_Pack/Particles/Parts/P_E_Sparks_03.P_E_Sparks_03" (`SceneComponent.K2_GetComponentLocation` _returnvalue) (`SceneComponent.K2_GetComponentRotation` _returnvalue) (`self.火花大小`)))

(fn `UserConstructionScript`)

(fn `获取对象引用`
  (returns (`角色基类` :type "/Game/_Game/Blueprints/角色基类 Object Reference"))
  (return null))